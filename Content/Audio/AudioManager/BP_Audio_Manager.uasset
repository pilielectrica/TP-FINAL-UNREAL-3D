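; BP_Audio_Manager is an audio manager actor that plays the game's music and a healing sound.
; On BeginPlay it starts a single Audio component, and the general and enemy music events switch tracks by setting opposite Play_General and Play_Enemy boolean parameters on it.
; Separate events stop the music or play the HealingSound component.
; The general music event also prints a Spanish debug message.
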(event `self.ReceiveBeginPlay`
  (`AudioComponent.Play` (`self.Audio`) 0.0))

(event `/Game/Audio/AudioManager/BPI_Audio.Play_General_Music`
  (`AudioComponent.SetBoolParameter` (`self.Audio`) "Play_Enemy" false)
  (`AudioComponent.SetBoolParameter` (`self.Audio`) "Play_General" true)
  (`KismetSystemLibrary.PrintString` "se llamo a la funcion musica general"))

(event `/Game/Audio/AudioManager/BPI_Audio.Play_Enemy_Music`
  (`AudioComponent.SetBoolParameter` (`self.Audio`) "Play_Enemy" true)
  (`AudioComponent.SetBoolParameter` (`self.Audio`) "Play_General" false))

(event `/Game/Audio/AudioManager/BPI_Audio.Stop_Music`
  (`AudioComponent.Stop` (`self.Audio`)))

(event `/Game/Audio/AudioManager/BPI_Audio.Play_Healing_Sound`
  (`AudioComponent.Play` (`self.healing sound`) 0.0))

(fn `UserConstructionScript`)