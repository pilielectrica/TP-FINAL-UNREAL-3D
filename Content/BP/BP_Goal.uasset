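; BP_Goal is the level's goal trigger, which ends the game when the player character overlaps it with enough fairies collected.
; On overlap by BPC_Character_UMG it asks the game mode for the fairy count and continues only when it equals three.
; It then plays the Fairys_Ending3 level sequence, stops the music through BP_Audio_Manager, and calls the HUD's game-over message when the sequence finishes.
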(event `self.ReceiveActorBeginOverlap`
  (params (OtherActor :type "Actor Object Reference"))
  (cast `/Game/Characters/BPC_Character_UMG` OtherActor)
  (bind _total_fairyies (message `/Game/BP/UI/Core/BPI_Game.Count_Fairyies` (`GameplayStatics.GetGameMode`)))
  (if (== _total_fairyies 3)
    (bind (_outactor _returnvalue) (`LevelSequencePlayer.CreateLevelSequencePlayer` "/Game/Cynematics/Fairys_Ending3.Fairys_Ending3"))
    (`MovieSceneSequencePlayer.Play` _returnvalue)
    (bind _returnvalue_2 (`GameplayStatics.GetActorOfClass` "/Game/Audio/MS/AudioManager/BP_Audio_Manager.BP_Audio_Manager_C"))
    (message `/Game/Audio/MS/AudioManager/BPI_Audio.Stop_Music` _returnvalue_2)
    (add `MovieSceneSequencePlayer.OnFinished` _returnvalue (delegate `volver al menu`))
    (else
      (`KismetSystemLibrary.PrintString` (`KismetStringLibrary.Conv_IntToString` 0)))))

(event `volver al menu`
  (message `/Game/BP/UI/Core/BPI_Game.GameOver` (`PlayerController.GetHUD` (`GameplayStatics.GetPlayerController` 0))))

(fn `UserConstructionScript`)