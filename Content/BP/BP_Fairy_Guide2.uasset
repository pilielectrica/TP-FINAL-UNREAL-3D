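; Fairy guide NPC that wanders the level until freed, then flies off to a checkpoint.
; While captive, it loops AI moves to random reachable nearby points, with a movement-updated callback turning it toward its destination at a yaw offset.
; FreeFairy stops the wandering, plays audio and the Fayri2_Fly level sequence, notifies the game mode, and teleports the fairy to a hard-coded location when the sequence finishes.
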(event `rotation` :!signature `self.OnCharacterMovementUpdated`
  (params (DeltaSeconds :type "Float (single-precision)") (OldLocation :type "Vector Structure") (OldVelocity :type "Vector Structure"))
  (if (not (`self.IsFree`))
    (`self.K2_SetActorRotation` (`KismetMathLibrary.MakeRotator` 0.0 0.0 (+ (.yaw (`KismetMathLibrary.FindLookAtRotation` (`self.K2_GetActorLocation`) (`self.Random Location`))) 200.0)))))

(event `FlyToCheckpoint`
  (bind (_outactor _returnvalue) (`LevelSequencePlayer.CreateLevelSequencePlayer` "/Game/Cynematics/Fayri2_Fly.Fayri2_Fly"))
  (`MovieSceneSequencePlayer.Play` _returnvalue)
  (`AudioComponent.Play` (`self.Audio`) 0.0)
  (add `MovieSceneSequencePlayer.OnFinished` _returnvalue (delegate `on finished`)))

(event `on finished`
  (`self.K2_SetActorLocation` (3970.0 5580.0 130.000003) false true))

(event `Move NPC`
  (if (not (`self.IsFree`))
    (bind _output_get (set `self.Random Location` (`NavigationSystemV1.K2_GetRandomReachablePointInRadius` (`self.K2_GetActorLocation`) 300.0 null null)))
    (`|AIMoveTo` self _output_get null 20.0
      (:`then`
        (set `self.Moving` true))
      (:`OnSuccess`
        (set `self.Moving` false)
        (`KismetSystemLibrary.Delay` 1.0)
        (`self.Move NPC` :!label _label)
        (add `self.OnCharacterMovementUpdated` (delegate `rotation`)))
      (:`OnFail`
        (set `self.Moving` false)
        (`KismetSystemLibrary.Delay` 2.0)
        (goto _label)))))

(event `self.ReceiveBeginPlay`
  (`self.Move NPC`))

(event `self.FreeFairy`
  (set `self.IsFree` true)
  (`self.FlyToCheckpoint`)
  (message `/Game/BP/UI/Core/BPI_Game.Add_Fairy` (`GameplayStatics.GetGameMode`)))

(fn `Add_Fairy`
  (returns (Total_Fayries :type Integer))
  (return 0))

(fn `Count_Fairyies`
  (returns (Total_Fairyies :type Integer))
  (return 0))

(fn `UserConstructionScript`)