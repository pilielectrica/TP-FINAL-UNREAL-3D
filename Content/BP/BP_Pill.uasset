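; BP_Pill is a health pickup that heals a BPC_Character_UMG that overlaps it, then destroys itself.
; On overlap it calls the character's restore-health message, passes the returned value divided by 100 to the player HUD, and plays a healing sound through a BP_Audio_Manager cached at BeginPlay.
; A debug "Hello" print remains, and the health and fairy-count functions are empty stubs returning zero.
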(event `self.ReceiveBeginPlay`
  (bind _returnvalue (`GameplayStatics.GetActorOfClass` "/Game/Audio/AudioManager/BP_Audio_Manager.BP_Audio_Manager_C"))
  (set `self.Audio_Manager_Ref` _returnvalue))

(event `self.ReceiveActorBeginOverlap`
  (params (OtherActor :type "Actor Object Reference"))
  (bind _asbpc_character_umg (cast `/Game/Characters/BPC_Character_UMG` OtherActor))
  (bind _newparam (message `/Game/BP/UI/Core/BPI_Restore_Health.Restore_Health` _asbpc_character_umg))
  (message `/Game/BP/UI/Core/BPI_Hud.Update Health` (`PlayerController.GetHUD` (`GameplayStatics.GetPlayerController` 0)) (/ _newparam 100.0))
  (message `/Game/Audio/AudioManager/BPI_Audio.Play_Healing_Sound` (`self.Audio_Manager_Ref`))
  (`KismetSystemLibrary.PrintString` "Hello")
  (`self.K2_DestroyActor`))

(fn `Add_Fairy`
  (returns (Total_Fayries :type Integer))
  (return 0))

(fn `Count_Fairyies`
  (returns (Total_Fairyies :type Integer))
  (return 0))

(fn `GetHealth`
  (returns (Value :type "Float (double-precision)"))
  (return 0.0))

(fn `GetHealthInPercent`
  (returns (Value :type "Float (double-precision)"))
  (return 0.0))

(fn `UserConstructionScript`)